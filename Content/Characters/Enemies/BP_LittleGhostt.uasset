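; Little ghost enemy that turns to face the player every tick and is destroyed when snowed.
; On spawn it registers with an overlapping BP_EnemyCollision and flags its blackboard as able to attack and having seen the player.
; AttackTimer runs a timed cooldown through the CanAttack key, while UpdateLittleHome stores its home there.
; An order event (Prikazed_1) spawns more little ghosts at random reachable points nearby.
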(event `self.ReceiveBeginPlay`
  (`self.CheckEnemyCollision`)
  (`KismetSystemLibrary.Delay` 0.2)
  (`BlackboardComponent.SetValueAsBool` (`AIBlueprintHelperLibrary.GetBlackboard` null) "CanAttack" true)
  (`BlackboardComponent.SetValueAsBool` (`AIBlueprintHelperLibrary.GetBlackboard` null) "HasSeenThePlayer?" true))

(event `self.ReceiveTick`
  (params (DeltaSeconds :type "Float (single-precision)"))
  (`self.Watch`))

(event `Watch`
  (`self.K2_SetActorRotation` (`KismetMathLibrary.FindLookAtRotation` (`self.K2_GetActorLocation`) (`self.K2_GetActorLocation` (`GameplayStatics.GetPlayerCharacter` 0)))))

(event `CheckEnemyCollision`
  (bind _asbp_enemy_collision (cast `/Game/ThirdPerson/Blueprints/LevelPrototyping/BP_EnemyCollision` (`|GetArrayItem` (`PrimitiveComponent.GetOverlappingActors` (`self.CapsuleComponent`) "/Game/ThirdPerson/Blueprints/LevelPrototyping/BP_EnemyCollision.BP_EnemyCollision_C"))))
  (`KismetArrayLibrary.Array_Add` (`/Game/ThirdPerson/Blueprints/LevelPrototyping/BP_EnemyCollision.LittleGhosts` _asbp_enemy_collision) self))

(event `Snowed`
  ;[0.5153 0.918 1] Снег
  (`self.K2_DestroyActor`))

(event `slingshoted`)

(event `SpawnGhost`
  ;[1 1 1] Приказ
  (`AIBlueprintHelperLibrary.SpawnAIFromClass` "BP_LittleGhostt_C" null (+ (`NavigationSystemV1.K2_GetRandomReachablePointInRadius` (`self.K2_GetActorLocation`) 200.0 null null) (* (`KismetMathLibrary.GetUpVector` (struct)) 100.0)) (struct) false null))

(event `AttackTimer`
  ;[1 1 1] Атака
  (if (`BlackboardComponent.GetValueAsBool` (`AIBlueprintHelperLibrary.GetBlackboard` null) "CanAttack")
    (`BlackboardComponent.SetValueAsBool` (`AIBlueprintHelperLibrary.GetBlackboard` null) "CanAttack" false)
    (`KismetSystemLibrary.PrintString` "Hello")
    (`KismetSystemLibrary.K2_SetTimerDelegate` (delegate `AttackAgain`) 5.0)))

(event `Prikazed_1`
  ;[1 1 1] Приказ
  (for _ (range 3)
    (`self.SpawnGhost`)))

(event `AttackAgain`
  ;[1 1 1] Атака
  (`BlackboardComponent.SetValueAsBool` (`AIBlueprintHelperLibrary.GetBlackboard` null) "CanAttack" true)
  (`KismetSystemLibrary.PrintString` "Hello" true true (struct :`R` 1.0 :`G` 0.317569 :`B` 0.381333 :`A` 1.0)))

(event `UpdateLittleHome`
  (params (LittleHome :type "/Game/ThirdPerson/Blueprints/BP_LittleHome Object Reference"))
  (`BlackboardComponent.SetValueAsObject` (`AIBlueprintHelperLibrary.GetBlackboard` null) "LittleHome" LittleHome))

(fn `UserConstructionScript`
  (`parent.UserConstructionScript`))