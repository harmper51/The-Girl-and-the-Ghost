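; BP_NormalGhostt is a ghost enemy character that spots the player and turns to oppose their facing.
; On BeginPlay it caches the overlapping BP_EnemyCollision volume, and incoming damage lowers Health with no death handling here.
; PawnSensing sets a blackboard flag on seeing BP_ThirdPersonDevochka, after which Tick sets yaw to the player's plus 180 degrees.
; Fire is an empty stub, and the BP_NewSnowball spawn is unconnected.
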(event `self.ReceiveBeginPlay`
  (bind _asbp_enemy_collision (cast `/Game/ThirdPerson/Blueprints/LevelPrototyping/BP_EnemyCollision` (`|GetArrayItem` (`PrimitiveComponent.GetOverlappingActors` (`self.CapsuleComponent`) "/Game/ThirdPerson/Blueprints/LevelPrototyping/BP_EnemyCollision.BP_EnemyCollision_C"))))
  (set `self.EnemiesInBoxCounter` _asbp_enemy_collision))

(event `self.ReceiveAnyDamage`
  (params (Damage :type "Float (single-precision)") (DamageType :type "DamageType Object Reference") (InstigatedBy :type "Controller Object Reference") (DamageCauser :type "Actor Object Reference"))
  (set `self.Health` (- (`self.Health`) Damage)))

(event `self.PawnSensing.OnSeePawn`
  (params (Pawn :type "Pawn Object Reference"))
  (cast `/Game/ThirdPerson/Blueprints/BP_ThirdPersonDevochka` Pawn)
  (`BlackboardComponent.SetValueAsBool` (`AIBlueprintHelperLibrary.GetBlackboard` (`self.GetController`)) "HasSeenThePlayer?" true))

(event `Fire`)

(event `self.ReceiveTick`
  (params (DeltaSeconds :type "Float (single-precision)"))
  (bind (_returnvalue_roll _returnvalue_pitch) (`KismetMathLibrary.BreakRotator` (`self.K2_GetActorRotation`)))
  (bind (_returnvalue_roll_2 _returnvalue_pitch_2 _returnvalue_yaw) (`KismetMathLibrary.BreakRotator` (`self.K2_GetActorRotation` (`GameplayStatics.GetPlayerCharacter` 0))))
  ;[1 1 1] Смотреть на игрока
  (if (`BlackboardComponent.GetValueAsBool` (`AIBlueprintHelperLibrary.GetBlackboard` (`self.GetController`)) "HasSeenThePlayer?")
    (`self.K2_SetActorRotation` (`KismetMathLibrary.MakeRotator` _returnvalue_roll _returnvalue_pitch (+ _returnvalue_yaw 180.0)))))

(fn `UserConstructionScript`
  (`parent.UserConstructionScript`))