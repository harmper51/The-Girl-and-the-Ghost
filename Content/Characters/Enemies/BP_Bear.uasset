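; Bear enemy that telegraphs a melee attack, exposing two paw weak points while it prepares.
; Timers turn it toward the player, lock rotation, then spawn a damage collision, with cooldown and hit state written to the AI Blackboard.
; An overlap during wind-up destroys that paw and interrupts preparation; losing both heals the player, spawns loot and destroys the bear.
; Slingshot reactions outside those states aggro it and damage the player.
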(event `AttackPrepare`
  ;[1 1 1] Атака
  (set `self.IsPreparing` true)
  (bind _returnvalue (`KismetSystemLibrary.K2_SetTimerDelegate` (delegate `SetRotation`) 0.1 true))
  (set `self.NewVar_0` _returnvalue)
  (`self.AttackTimer`)
  (`SceneComponent.SetVisibility` (`self.Hand1`) true false)
  (`SceneComponent.SetVisibility` (`self.Hand2`) true false)
  (`KismetSystemLibrary.K2_SetTimerDelegate` (delegate `StopRotation`) 3.0))

(event `SetRotation`
  (bind (_returnvalue_roll _returnvalue_pitch) (`KismetMathLibrary.BreakRotator` (`self.K2_GetActorRotation`)))
  (bind (_returnvalue_roll_2 _returnvalue_pitch_2 _returnvalue_yaw) (`KismetMathLibrary.BreakRotator` (`KismetMathLibrary.FindLookAtRotation` (`self.K2_GetActorLocation`) (`self.K2_GetActorLocation` (`GameplayStatics.GetPlayerCharacter` 0)))))
  ;[1 1 1] Атака
  (`self.K2_SetActorRotation` (`KismetMathLibrary.MakeRotator` _returnvalue_roll _returnvalue_pitch _returnvalue_yaw)))

(event `StopRotation`
  ;[1 1 1] Атака
  (`KismetSystemLibrary.K2_ClearAndInvalidateTimerHandle` (`self.NewVar_0`))
  (`KismetSystemLibrary.K2_SetTimerDelegate` (delegate `TimeToAttack`) 0.8))

(event `self.ReceiveBeginPlay`
  (`BlackboardComponent.SetValueAsBool` (`AIBlueprintHelperLibrary.GetBlackboard` null) "CanAttack" true))

(event `TimeToAttack`
  ;[1 1 1] Атака
  (`SceneComponent.SetVisibility` (`self.Hand1`) false false)
  (`SceneComponent.SetVisibility` (`self.Hand2`) false false)
  (`|SpawnActorFromClass` "/Game/Characters/Enemies/BEAR/BearDamage_Collision.BearDamage_Collision_C" (`KismetMathLibrary.Conv_VectorToTransform` (`SceneComponent.K2_GetComponentLocation` (`self.Arrow2`))) "Undefined" "MultiplyWithRoot" self null)
  (set `self.IsPreparing` false))

(event `self.IsSnowed Custom`
  ;[0.3142 0.8536 1] Снег
)

(event `self.SlingshotReaction`
  ;[1 0.3247 0.3187] Рогатка
  (if (`self.IsPreparing`)
    _
    (elif (not (`self.IsBeingShot`))
      (`BlackboardComponent.SetValueAsBool` (`AIBlueprintHelperLibrary.GetBlackboard` null) "HasSeenThePlayer?" true)
      (`GameplayStatics.ApplyDamage` (`GameplayStatics.GetPlayerCharacter` 0) 5.0))))

(event `self.Prikazed`
  ;[1 1 1] Приказ
)

(event `Rotate Bear`
  (bind (_returnvalue_roll _returnvalue_pitch) (`KismetMathLibrary.BreakRotator` (`self.K2_GetActorRotation`)))
  ;[1 1 1] Поворот во время атаки
  (set `self.StartRotation` (`self.K2_GetActorRotation`))
  (set `self.Rotator` (`KismetMathLibrary.FindLookAtRotation` (`self.K2_GetActorLocation`) (`self.K2_GetActorLocation` (`GameplayStatics.GetPlayerCharacter` 0))))
  (bind (_direction _alpha) (`Timeline|Timeline`)
    (:`Update`
      (`self.K2_SetActorRotation` (`KismetMathLibrary.MakeRotator` _returnvalue_roll _returnvalue_pitch (`KismetMathLibrary.Lerp` (.yaw (`self.StartRotation`)) (.yaw (`self.Rotator`)) _alpha))))))

(event `self.Hand2.OnComponentBeginOverlap`
  (params (OverlappedComponent :type "PrimitiveComponent Object Reference") (OtherActor :type "Actor Object Reference") (OtherComp :type "PrimitiveComponent Object Reference") (OtherBodyIndex :type Integer) (bFromSweep :type Boolean) (SweepResult :type "HitResult Structure (by ref)"))
  (if (`self.IsPreparing`)
    (`KismetArrayLibrary.Array_RemoveItem` (`self.Hands`) "Hand2")
    (`ActorComponent.K2_DestroyComponent` OverlappedComponent)
    (set `self.LeftPawShot` true)
    (set `self.IsBeingShot` true :!label _label)
    (set `self.IsPreparing` false)
    (`BlackboardComponent.SetValueAsBool` (`AIBlueprintHelperLibrary.GetBlackboard` (`self.GetController`)) "IsShot!" true)
    (`SkeletalMeshComponent.PlayAnimation` (`self.Mesh`) "/Game/Characters/Enemies/EnemyAss/Bear/BEAR_Anim_metarig_metarig_Scene.BEAR_Anim_metarig_metarig_Scene" true)
    (`KismetSystemLibrary.K2_SetTimerDelegate` (delegate `NotShotAgain`) 2.0)
    (`self.TimeToDie`)))

(event `self.Hand1.OnComponentBeginOverlap`
  (params (OverlappedComponent :type "PrimitiveComponent Object Reference") (OtherActor :type "Actor Object Reference") (OtherComp :type "PrimitiveComponent Object Reference") (OtherBodyIndex :type Integer) (bFromSweep :type Boolean) (SweepResult :type "HitResult Structure (by ref)"))
  (if (`self.IsPreparing`)
    (`KismetArrayLibrary.Array_RemoveItem` (`self.Hands`) "Hand1")
    (`ActorComponent.K2_DestroyComponent` OverlappedComponent)
    (set `self.RightPawShot` true)
    (goto _label)))

(event `NotShotAgain`
  (set `self.IsBeingShot` false)
  (`/Engine/EditorBlueprintResources/StandardMacros.IsValid` (`self.GetController`)
    (:`Is Valid`
      (`BlackboardComponent.SetValueAsBool` (`AIBlueprintHelperLibrary.GetBlackboard` (`self.GetController`)) "IsShot!" false))))

(event `AttackTimer`
  ;[1 1 1] Attack Timer
  (if (`BlackboardComponent.GetValueAsBool` (`AIBlueprintHelperLibrary.GetBlackboard` null) "CanAttack")
    (`BlackboardComponent.SetValueAsBool` (`AIBlueprintHelperLibrary.GetBlackboard` null) "CanAttack" false)
    (bind _returnvalue (`KismetSystemLibrary.K2_SetTimerDelegate` (delegate `AttackAgain`) 9.0))
    (set `self.NewVar_1` _returnvalue)))

(event `AttackAgain`
  ;[1 1 1] Attack Timer
  (`BlackboardComponent.SetValueAsBool` (`AIBlueprintHelperLibrary.GetBlackboard` null) "CanAttack" true))

(event `self.TimeToDie`
  (bind _as_bp_enemy_collision (`self.As BP Enemy Collision`))
  ;[1 1 1] Смерть
  (if (<= (`KismetArrayLibrary.Array_Length` (`self.Hands`)) 0)
    (`/Game/ThirdPerson/Blueprints/BP_ThirdPersonDevochka.Heal Devochka` (cast `/Game/ThirdPerson/Blueprints/BP_ThirdPersonDevochka` (`GameplayStatics.GetPlayerCharacter` 0) :!pure true) (`self.HowMuchHeal`))
    (set `/Game/ThirdPerson/Blueprints/LevelPrototyping/BP_EnemyCollision.EnemyLocation` (`self.K2_GetActorLocation`) _as_bp_enemy_collision)
    (`/Game/ThirdPerson/Blueprints/LevelPrototyping/BP_EnemyCollision.SpawnLoot` _as_bp_enemy_collision)
    (`self.K2_DestroyActor`)))

(event `Play Animation`
  (params (Location :type "Vector Structure"))
  (`GameplayStatics.SpawnEmitterAtLocation` "/Game/Characters/Devochka/FX/death.death" Location))

(fn `Count Enemies`
  (returns (ReturnValue :type Boolean))
  (set `self.NewLocalVar` 0)
  (for _array_element (`PrimitiveComponent.GetOverlappingActors` (`/Game/ThirdPerson/Blueprints/LevelPrototyping/BP_EnemyCollision.Box` (`self.As BP Enemy Collision`)) "/Game/Characters/Enemies/BP_EnemyBase.BP_EnemyBase_C")
    (`/Engine/EditorBlueprintResources/StandardMacros.IsValid` _array_element
      (:`Is Valid`
        (`/Engine/EditorBlueprintResources/StandardMacros.IncrementInt` (`self.NewLocalVar`)))))
  (return (<= (`self.NewLocalVar`) 4)))

(fn `IsDevockaWatching?`
  (returns (`IsWatching?` :type Boolean))
  (bind _followcamera (`/Game/ThirdPerson/Blueprints/BP_ThirdPersonDevochka.FollowCamera` (cast `/Game/ThirdPerson/Blueprints/BP_ThirdPersonDevochka` (`GameplayStatics.GetPlayerCharacter` 0) :!pure true)))
  (bind _returnvalue (`SceneComponent.GetForwardVector` _followcamera))
  (bind _returnvalue_2 (`KismetMathLibrary.Normal` (- (`self.K2_GetActorLocation`) (`SceneComponent.K2_GetComponentLocation` _followcamera))))
  (return (< (`KismetMathLibrary.Acos` (/ (+ (* (.x _returnvalue) (.x _returnvalue_2)) (* (.y _returnvalue) (.y _returnvalue_2)) (* (.z _returnvalue) (.z _returnvalue_2))) (* (`KismetMathLibrary.VSize` _returnvalue_2) (`KismetMathLibrary.VSize` _returnvalue)))) 1.0)))

(fn `UserConstructionScript`
  (`parent.UserConstructionScript`))