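; Tutorial squirrel enemy that reacts by throwing an acorn (BP_Jelud) at the player and triggers tutorial voice lines.
; CustomReaction runs only until TutorialDialogueDone is set, playing a one-time slingshot line, clearing a timer and firing the acorn.
; Prikazed spawns a ghost and destroys the actor, first hiding the mesh during a voice-line delay if the tutorial is unfinished.
; VoicelinesController's ActiveCue serves as a shared lock against overlapping lines.
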(event `/Game/Characters/Enemies/BP_EnemyBase.CustomReaction`
  (bind _returnvalue (`self.K2_GetActorLocation`))
  (bind _sound_to_play (`self.Sound to play`))
  (if (not (`/Game/ThirdPerson/DevochkaInstance.TutorialDialogueDone` (cast `/Game/ThirdPerson/DevochkaInstance` (`GameplayStatics.GetGameInstance`) :!pure true)))
    (bind _returnvalue_2 (`GameplayStatics.GetActorOfClass` "/Game/Noises/VoicelinesController.VoicelinesController_C"))
    (`/Engine/EditorBlueprintResources/StandardMacros.IsValid` (`/Game/Noises/VoicelinesController.Active Cue` _returnvalue_2)
      (:`Is Valid`
        _)
      (:`Is Not Valid`
        ;[1 0.3247 0.3187] Рогатка
        (set `/Game/Noises/VoicelinesController.Active Cue` _sound_to_play _returnvalue_2)
        (`/Engine/EditorBlueprintResources/StandardMacros.DoOnce` false
          (:`Completed`
            (`GameplayStatics.PlaySound2D` _sound_to_play 1.0 1.0 0.0 null null)))))
    (`KismetSystemLibrary.K2_ClearAndInvalidateTimerHandle` (`self.NewVar_0`))
    (`SkeletalMeshComponent.PlayAnimation` (`self.Mesh`) "/Game/Characters/Enemies/EnemyAss/Squirrel/squirrel_Anim_metarig_Throw.squirrel_Anim_metarig_Throw" false) ; анимация получения урона
    (`|SpawnActorFromClass` "/Game/ThirdPerson/Blueprints/Guns/BP_Jelud.BP_Jelud_C" (`KismetMathLibrary.MakeTransform` _returnvalue (`KismetMathLibrary.FindLookAtRotation` _returnvalue (`self.K2_GetActorLocation` (`GameplayStatics.GetPlayerCharacter` 0)))) "Undefined" "MultiplyWithRoot" null null)))

(event `/Game/Characters/Enemies/BP_EnemyBase.Prikazed`
  (bind _mesh (`self.Mesh`))
  (for _ (range 2)
    (`self.SpawnGhost`)
    (if (`/Game/ThirdPerson/DevochkaInstance.TutorialDialogueDone` (cast `/Game/ThirdPerson/DevochkaInstance` (`GameplayStatics.GetGameInstance`) :!pure true))
      (`self.K2_DestroyActor`)
      (else
        (`/Engine/EditorBlueprintResources/StandardMacros.IsValid` _mesh
          (:`Is Valid`
            (`SceneComponent.SetVisibility` _mesh false false))
          (:`Is Not Valid`
            _))
        (bind _returnvalue (`GameplayStatics.GetActorOfClass` "/Game/Noises/VoicelinesController.VoicelinesController_C"))
        (`/Engine/EditorBlueprintResources/StandardMacros.IsValid` (`/Game/Noises/VoicelinesController.Active Cue` _returnvalue)
          (:`Is Valid`
            (`KismetSystemLibrary.Delay` 3.0)
            (set `/Game/Noises/VoicelinesController.Active Cue` null _returnvalue))
          (:`Is Not Valid`
            (bind _output_get (set `/Game/Noises/VoicelinesController.Active Cue` (`self.Sound to play_0`) _returnvalue))
            (`GameplayStatics.PlaySound2D` _output_get 1.0 1.0 0.0 null null)
            (`KismetSystemLibrary.Delay` 4.0)
            (set `/Game/Noises/VoicelinesController.Active Cue` null _returnvalue)))
        (`self.K2_DestroyActor`)))))

(fn `UserConstructionScript`
  (`parent.UserConstructionScript`))