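; Tutorial variant of the strong ghost enemy that turns into a normal ghost when it is snowed.
; While tutorial dialogue is unfinished, IsSnowed claims the VoicelinesController's active cue, if free, and plays a 2D voiceline once.
; It plays a throw montage and stops movement, then after a short delay spawns BP_NormalGhost with its behavior tree and a particle burst.
; It then clears the active cue and destroys itself.
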(event `/Game/Characters/Enemies/BP_EnemyBase.IsSnowed`
  (bind (_returnvalue_location _returnvalue_rotation) (`KismetMathLibrary.BreakTransform` (`self.GetTransform`)))
  (bind _sound_to_play (`self.Sound to play`))
  (if (not (`/Game/ThirdPerson/DevochkaInstance.TutorialDialogueDone` (cast `/Game/ThirdPerson/DevochkaInstance` (`GameplayStatics.GetGameInstance`) :!pure true)))
    (bind _returnvalue (`GameplayStatics.GetActorOfClass` "/Game/Noises/VoicelinesController.VoicelinesController_C"))
    (`/Engine/EditorBlueprintResources/StandardMacros.IsValid` (`/Game/Noises/VoicelinesController.Active Cue` _returnvalue)
      (:`Is Valid`
        _)
      (:`Is Not Valid`
        (set `/Game/Noises/VoicelinesController.Active Cue` _sound_to_play _returnvalue)
        (`/Engine/EditorBlueprintResources/StandardMacros.DoOnce` false
          (:`Completed`
            (`GameplayStatics.PlaySound2D` _sound_to_play 1.0 1.0 0.0 null null)))))
    (`/Engine/EditorBlueprintResources/StandardMacros.DoOnce` false
      (:`Completed`
        _)))
  (`|PlayMontage` (`self.Mesh`) "/Game/Characters/Enemies/EnemyAss/SheetGhost/sheetghost_Anim_Armatur_Throw_Montage.sheetghost_Anim_Armatur_Throw_Montage"
    (:`then`
      (`CharacterMovementComponent.DisableMovement` (`self.CharacterMovement`))
      (`KismetSystemLibrary.Delay` 1.0)
      (`AIBlueprintHelperLibrary.SpawnAIFromClass` "/Game/Characters/Enemies/BP_NormalGhost.BP_NormalGhost_C" "/Game/Characters/Enemies/Behaviour_Trees/BehaviorTree_NormalGhost.BehaviorTree_NormalGhost" _returnvalue_location _returnvalue_rotation false null)
      (`GameplayStatics.SpawnEmitterAtLocation` "/Game/Characters/Devochka/FX/NewParticleSystem3.NewParticleSystem3" (+ (`self.K2_GetActorLocation`) (0.0 0.0 50.0)) (struct) (0.5 0.5 0.5))
      (set `/Game/Noises/VoicelinesController.Active Cue` null _returnvalue)
      (`self.K2_DestroyActor`))))

(fn `UserConstructionScript`
  (`parent.UserConstructionScript`))