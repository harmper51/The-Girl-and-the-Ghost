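; Squirrel enemy character that throws acorns at the player, summons ghosts and reacts to slingshot and snow hits.
; A blackboard CanAttack flag and timer gate attacks, while slingshot hits reset the cooldown and fire an acorn back at the player.
; An order event spawns BP_NormalGhost at random reachable points nearby.
; A camera-angle check detects whether the player is watching, while Tick calls Watch and debug-prints that angle.
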(event `self.CustomReaction`
  (bind _returnvalue (`self.K2_GetActorLocation`))
  ;[1 0.3247 0.3187] Рогатка
  (`BlackboardComponent.SetValueAsBool` (`AIBlueprintHelperLibrary.GetBlackboard` null) "CanAttack" true)
  (`KismetSystemLibrary.K2_ClearAndInvalidateTimerHandle` (`self.NewVar`))
  (`SkeletalMeshComponent.PlayAnimation` (`self.Mesh`) "/Game/Characters/Enemies/EnemyAss/Squirrel/squirrel_Anim_metarig_Throw.squirrel_Anim_metarig_Throw" false) ; анимация получения урона
  (`GameplayStatics.PlaySound2D` null 1.0 1.0 0.0 null null) ; звук получения урона
  (`|SpawnActorFromClass` "/Game/ThirdPerson/Blueprints/Guns/BP_Jelud.BP_Jelud_C" (`KismetMathLibrary.MakeTransform` _returnvalue (`KismetMathLibrary.FindLookAtRotation` _returnvalue (`self.K2_GetActorLocation` (`GameplayStatics.GetPlayerCharacter` 0)))) "Undefined" "MultiplyWithRoot" null null))

(event `self.ReceiveTick`
  (params (DeltaSeconds :type "Float (single-precision)"))
  (bind _followcamera (`/Game/ThirdPerson/Blueprints/BP_ThirdPersonDevochka.FollowCamera` (cast `/Game/ThirdPerson/Blueprints/BP_ThirdPersonDevochka` (`GameplayStatics.GetPlayerCharacter` 0) :!pure true)))
  (bind _returnvalue (`SceneComponent.GetForwardVector` _followcamera))
  (bind _returnvalue_2 (`KismetMathLibrary.Normal` (- (`self.K2_GetActorLocation`) (`SceneComponent.K2_GetComponentLocation` _followcamera))))
  (`self.Watch`)
  (`KismetSystemLibrary.PrintString` (`KismetStringLibrary.Conv_DoubleToString` (`KismetMathLibrary.Acos` (/ (+ (* (.x _returnvalue) (.x _returnvalue_2)) (* (.y _returnvalue) (.y _returnvalue_2)) (* (.z _returnvalue) (.z _returnvalue_2))) (* (`KismetMathLibrary.VSize` _returnvalue_2) (`KismetMathLibrary.VSize` _returnvalue))))) true true (struct :`G` 0.66 :`B` 1.0 :`A` 1.0) 0.0))

(event `SpawnGhost`
  ;[1 1 1] Приказ
  (`AIBlueprintHelperLibrary.SpawnAIFromClass` "/Game/Characters/Enemies/BP_NormalGhost.BP_NormalGhost_C" null (+ (`NavigationSystemV1.K2_GetRandomReachablePointInRadius` (`self.K2_GetActorLocation`) 300.0 null null) (* (`KismetMathLibrary.GetUpVector` (struct)) 100.0)) (struct) false null))

(event `self.ReceiveBeginPlay`
  ;[1 1 1] Атака
  (`BlackboardComponent.SetValueAsBool` (`AIBlueprintHelperLibrary.GetBlackboard` null) "CanAttack" true))

(event `AttackTimer`
  ;[1 1 1] Атака
  (if (`BlackboardComponent.GetValueAsBool` (`AIBlueprintHelperLibrary.GetBlackboard` null) "CanAttack")
    (`BlackboardComponent.SetValueAsBool` (`AIBlueprintHelperLibrary.GetBlackboard` null) "CanAttack" false)
    (bind _returnvalue (`KismetSystemLibrary.K2_SetTimerDelegate` (delegate `AttackAgain`) 5.0))
    (set `self.NewVar` _returnvalue)))

(event `self.Prikazed Custom`
  ;[1 1 1] Приказ
  (for _ (range 2)
    (`self.SpawnGhost`)))

(event `AttackAgain`
  ;[1 1 1] Атака
  (`BlackboardComponent.SetValueAsBool` (`AIBlueprintHelperLibrary.GetBlackboard` null) "CanAttack" true))

(event `self.IsSnowed Custom`
  ;[0.3142 0.8536 1] Снег
  (`SkeletalMeshComponent.PlayAnimation` (`self.Mesh`) "/Game/Characters/Enemies/EnemyAss/Squirrel/squirrel_Anim_metarig_Throw.squirrel_Anim_metarig_Throw" false) ; анимация получения урона
  (`GameplayStatics.PlaySound2D` null 1.0 1.0 0.0 null null) ; звук получения урона
)

(fn `IsDevockaWatching?`
  (returns (`IsWatching?` :type Boolean))
  (bind _followcamera (`/Game/ThirdPerson/Blueprints/BP_ThirdPersonDevochka.FollowCamera` (cast `/Game/ThirdPerson/Blueprints/BP_ThirdPersonDevochka` (`GameplayStatics.GetPlayerCharacter` 0) :!pure true)))
  (bind _returnvalue (`SceneComponent.GetForwardVector` _followcamera))
  (bind _returnvalue_2 (`KismetMathLibrary.Normal` (- (`self.K2_GetActorLocation`) (`SceneComponent.K2_GetComponentLocation` _followcamera))))
  (return (< (`KismetMathLibrary.Acos` (/ (+ (* (.x _returnvalue) (.x _returnvalue_2)) (* (.y _returnvalue) (.y _returnvalue_2)) (* (.z _returnvalue) (.z _returnvalue_2))) (* (`KismetMathLibrary.VSize` _returnvalue_2) (`KismetMathLibrary.VSize` _returnvalue)))) 1.0)))

(fn `UserConstructionScript`
  (`parent.UserConstructionScript`))