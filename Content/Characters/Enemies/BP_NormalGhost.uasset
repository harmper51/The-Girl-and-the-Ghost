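; Normal ghost enemy with two health that runs inherited aggro and watch logic and registers its overlapping BP_EnemyCollision as enemy counter.
; Slingshot hits cost health, play a montage, call TimeToDie, briefly halt movement and flag the player as seen on the blackboard.
; Snow replaces the ghost with an ice statue.
; The Prikazed (order) event spawns two more AI-driven ghosts at random reachable points nearby.
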(event `self.ReceiveBeginPlay`
  (`self.StartAgritsa`)
  (set `self.Health` 2)
  (bind _asbp_enemy_collision (cast `/Game/ThirdPerson/Blueprints/LevelPrototyping/BP_EnemyCollision` (`|GetArrayItem` (`PrimitiveComponent.GetOverlappingActors` (`self.CapsuleComponent`) "/Game/ThirdPerson/Blueprints/LevelPrototyping/BP_EnemyCollision.BP_EnemyCollision_C"))))
  (set `self.EnemiesInBoxCounter` _asbp_enemy_collision)
  (`self.StartAgritsa`))

(event `self.ReceiveTick`
  (params (DeltaSeconds :type "Float (single-precision)"))
  (`self.Watch`))

(event `self.IsSnowed`
  ;[0.5153 0.918 1] Снег
  (`|SpawnActorFromClass` "/Game/Characters/Enemies/BP_IceStatue.BP_IceStatue_C" (`self.GetTransform`) "AlwaysSpawn" "MultiplyWithRoot" null null)
  (`self.K2_DestroyActor`))

(event `self.SlingshotReaction`
  ;[1 0.3652 0.3433] Рогатка
  (set `self.Health` (- (`self.Health`) 1))
  (`|PlayMontage` (`self.Mesh`) "/Game/Characters/Enemies/EnemyAss/NormGhost/ghostnormal_Anim_Ghostarmature_Attac_Montage.ghostnormal_Anim_Ghostarmature_Attac_Montage"
    (:`then`
      (`CharacterMovementComponent.DisableMovement` (`self.CharacterMovement`))
      (`self.TimeToDie`)
      (`KismetSystemLibrary.Delay` 0.2)
      (`CharacterMovementComponent.SetMovementMode` (`self.CharacterMovement`) "MOVE_Walking" 0)
      (`BlackboardComponent.SetValueAsBool` (`AIBlueprintHelperLibrary.GetBlackboard` null) "HasSeenThePlayer?" true))))

(event `SpawnGhost`
  ;[1 1 1] Приказ
  (`AIBlueprintHelperLibrary.SpawnAIFromClass` "BP_NormalGhost_C" "/Game/Characters/Enemies/Behaviour_Trees/BehaviorTree_NormalGhost.BehaviorTree_NormalGhost" (+ (`NavigationSystemV1.K2_GetRandomReachablePointInRadius` (`self.K2_GetActorLocation`) 200.0 null null) (* (`KismetMathLibrary.GetUpVector` (struct)) 100.0)) (struct) false null))

(event `self.Prikazed`
  ;[1 1 1] Приказ
  (for _ (range 2)
    (`self.SpawnGhost`)))

(fn `UserConstructionScript`
  (`parent.UserConstructionScript`))