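; Strong ghost enemy that turns into a normal ghost when it gets snowed.
; The IsSnowed event runs once, playing the throw animation and disabling movement.
; After a short delay it spawns BP_NormalGhost with its behavior tree at the same location and rotation, then destroys itself.
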(event `self.IsSnowed`
  (bind (_returnvalue_location _returnvalue_rotation) (`KismetMathLibrary.BreakTransform` (`self.GetTransform`)))
  (`/Engine/EditorBlueprintResources/StandardMacros.DoOnce` false
    (:`Completed`
      (`SkeletalMeshComponent.PlayAnimation` (`self.Mesh`) "/Game/Characters/Enemies/EnemyAss/SheetGhost/sheetghost_Anim_Armatur_Throw.sheetghost_Anim_Armatur_Throw" false)
      (`CharacterMovementComponent.DisableMovement` (`self.CharacterMovement`))
      (`KismetSystemLibrary.Delay` 1.0)
      (`AIBlueprintHelperLibrary.SpawnAIFromClass` "/Game/Characters/Enemies/BP_NormalGhost.BP_NormalGhost_C" "/Game/Characters/Enemies/Controllers/BehaviorTree_NormalGhost.BehaviorTree_NormalGhost" _returnvalue_location _returnvalue_rotation false null)
      (`self.K2_DestroyActor`))))

(fn `UserConstructionScript`
  (`parent.UserConstructionScript`))