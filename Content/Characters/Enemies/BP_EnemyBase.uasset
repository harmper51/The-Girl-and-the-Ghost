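; Base enemy character that feeds player detection into its AI Blackboard once the player's battle has started.
; A looping line-trace timer and PawnSensing set the seen flag, while Turn clears it and Watch faces the player.
; TimeToDie heals the player, spawns loot and destroys the enemy at zero health.
; Reaction events are empty hooks, and the home-leash check HowFarAmI has its setup disconnected.
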(event `StartAgritsa`
  ;[1 1 1] Атаковать, когда игрок рядом
  (`KismetSystemLibrary.K2_SetTimerDelegate` (delegate `CheckHowFarPlayer`) 1.0 true))

(event `CheckHowFarPlayer`
  (bind _returnvalue (`self.K2_GetActorLocation`))
  ;[1 1 1] Атаковать, когда игрок рядом
  (if (`self.CanSeeAPlayer`)
    (bind _returnvalue_2 (`GameplayStatics.GetActorOfClass` "/Game/ThirdPerson/Blueprints/BP_ThirdPersonDevochka.BP_ThirdPersonDevochka_C"))
    (if (`/Game/ThirdPerson/Blueprints/BP_ThirdPersonDevochka.BattleStarted` _returnvalue_2)
      (bind (_outhit _returnvalue_3) (`KismetSystemLibrary.LineTraceSingle` :`Start` _returnvalue :`End` (+ _returnvalue (* (`KismetMathLibrary.Normal` (- (`self.K2_GetActorLocation` (`GameplayStatics.GetPlayerCharacter` 0)) _returnvalue)) (`self.HowFarISee`))) :`TraceChannel` "TraceTypeQuery2" :`DrawDebugType` "ForDuration" :`TraceColor` (struct :`R` 1.0 :`G` 0.031895 :`A` 1.0)))
      (if _returnvalue_3
        (cast `/Game/ThirdPerson/Blueprints/BP_ThirdPersonDevochka` (`.HitActor` (`GameplayStatics.BreakHitResult` _outhit)))
        (`BlackboardComponent.SetValueAsBool` (`AIBlueprintHelperLibrary.GetBlackboard` (`self.GetController`)) "HasSeenThePlayer?" true)))))

(event `self.ReceiveBeginPlay`
  (`self.StartAgritsa`))

(event `SlingshotReaction`
  ;[1 1 1] Рогатка
)

(event `TimeToDie`
  (bind _as_bp_enemy_collision (`self.As BP Enemy Collision`))
  ;[1 1 1] Рогатка
  (if (<= (`self.Health`) 0)
    (if (not (`self.IsGoingToDie`))
      (set `self.IsGoingToDie` true)
      (bind _returnvalue (`GameplayStatics.GetActorOfClass` "/Game/ThirdPerson/Blueprints/BP_ThirdPersonDevochka.BP_ThirdPersonDevochka_C"))
      (`/Game/ThirdPerson/Blueprints/BP_ThirdPersonDevochka.Heal Devochka` _returnvalue (`self.HowMuchHeal`))
      (`KismetSystemLibrary.Delay` 0.5))
    (`/Engine/EditorBlueprintResources/StandardMacros.IsValid` _as_bp_enemy_collision
      (:`Is Valid`
        (set `/Game/ThirdPerson/Blueprints/LevelPrototyping/BP_EnemyCollision.EnemyLocation` (`self.K2_GetActorLocation`) _as_bp_enemy_collision)
        (`/Game/ThirdPerson/Blueprints/LevelPrototyping/BP_EnemyCollision.SpawnLoot` _as_bp_enemy_collision))
      (:`Is Not Valid`
        _))
    (`self.K2_DestroyActor`)))

(event `CustomReaction`
  ;[1 1 1] Рогатка
)

(event `Prikazed`)

(event `Prikazed Custom`)

(event `DeleteEnemy`
  (`self.K2_DestroyActor`))

(event `IsSnowed`)

(event `IsSnowed Custom`)

(event `Turn`
  (params (IsActive :type Boolean))
  (bind _returnvalue (`AIBlueprintHelperLibrary.GetBlackboard` null))
  (bind _output_get (set `self.Is Active` IsActive))
  (`BlackboardComponent.SetValueAsBool` _returnvalue (`self.Key Name`) _output_get)
  ;[1 1 1] Comment
  (`BlackboardComponent.SetValueAsBool` _returnvalue "HasSeenThePlayer?" false)
  (if _output_get
    (`MovementComponent.StopMovementImmediately` (`self.CharacterMovement`))))

(event `HowFarAmI`
  (bind _homereference (`self.HomeReference`))
  (bind _returnvalue (`KismetMathLibrary.VSize` (- (`self.K2_GetActorLocation` _homereference) (`self.K2_GetActorLocation`))))
  (`/Engine/EditorBlueprintResources/StandardMacros.IsValid` _homereference
    (:`Is Valid`
      (if (<= (`KismetMathLibrary.VSize` (- (`self.K2_GetActorLocation`) (`self.K2_GetActorLocation` (`GameplayStatics.GetPlayerCharacter` 0)))) 400.0)
        (set `self.IsHome` true)
        (bind _output_get (set `self.ShouldGoHome` false))
        (`BlackboardComponent.SetValueAsBool` (`AIBlueprintHelperLibrary.GetBlackboard` (`self.GetController`)) "ShouldiGoHome" _output_get)
        (elif (>= _returnvalue 500.0)
          (set `self.IsHome` false)
          (`BlackboardComponent.SetValueAsBool` (`AIBlueprintHelperLibrary.GetBlackboard` (`self.GetController`)) "HasSeenThePlayer?" false)
          (bind _output_get_2 (set `self.ShouldGoHome` true))
          (`BlackboardComponent.SetValueAsBool` (`AIBlueprintHelperLibrary.GetBlackboard` (`self.GetController`)) "ShouldiGoHome" _output_get_2)
          (elif (<= _returnvalue 150.0)
            (set `self.IsHome` true)
            (bind _output_get_3 (set `self.ShouldGoHome` false))
            (`BlackboardComponent.SetValueAsBool` (`AIBlueprintHelperLibrary.GetBlackboard` (`self.GetController`)) "ShouldiGoHome" _output_get_3)))))))

(event `self.PawnSensing.OnSeePawn`
  (params (Pawn :type "Pawn Object Reference"))
  (if (`self.CanSeeAPlayer`)
    (if (not (`self.ShouldGoHome`))
      (bind _asbp_third_person_devochka (cast `/Game/ThirdPerson/Blueprints/BP_ThirdPersonDevochka` Pawn))
      (if (`/Game/ThirdPerson/Blueprints/BP_ThirdPersonDevochka.BattleStarted` _asbp_third_person_devochka)
        (`BlackboardComponent.SetValueAsBool` (`AIBlueprintHelperLibrary.GetBlackboard` (`self.GetController`)) "HasSeenThePlayer?" true)))))

(event `Watch`
  (bind _returnvalue (`AIBlueprintHelperLibrary.GetBlackboard` (`self.GetController`)))
  (`/Engine/EditorBlueprintResources/StandardMacros.IsValid` _returnvalue
    (:`Is Valid`
      (if (`self.Is Active`)
        _
        (elif (`BlackboardComponent.GetValueAsBool` _returnvalue "HasSeenThePlayer?")
          (`self.K2_SetActorRotation` (`KismetMathLibrary.FindLookAtRotation` (`self.K2_GetActorLocation`) (`self.K2_GetActorLocation` (`GameplayStatics.GetPlayerCharacter` 0)))))))))

(event `self.ReceiveTick`
  (params (DeltaSeconds :type "Float (single-precision)")))

(fn `UserConstructionScript`)