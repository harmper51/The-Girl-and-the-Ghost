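; Normal ghost enemy (Casper) Blueprint that defines how the ghost reacts to slingshot hits.
; Until tutorial dialogue is done, a hit can claim the VoicelinesController's free cue slot and play a one-time voiceline.
; The reaction plays an attack montage, briefly disables movement, then restores walking and spawns the Death particle effect.
; A second later it clears the active cue and destroys the ghost if Health equals one.
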(event `self.SlingshotReaction`
  (bind _sound_to_play (`self.Sound to play`))
  (if (not (`/Game/ThirdPerson/DevochkaInstance.TutorialDialogueDone` (cast `/Game/ThirdPerson/DevochkaInstance` (`GameplayStatics.GetGameInstance`) :!pure true)))
    (bind _returnvalue (`GameplayStatics.GetActorOfClass` "/Game/Noises/VoicelinesController.VoicelinesController_C"))
    (`/Engine/EditorBlueprintResources/StandardMacros.IsValid` (`/Game/Noises/VoicelinesController.Active Cue` _returnvalue)
      (:`Is Valid`
        _)
      (:`Is Not Valid`
        (set `/Game/Noises/VoicelinesController.Active Cue` _sound_to_play _returnvalue)
        (`/Engine/EditorBlueprintResources/StandardMacros.DoOnce` false
          (:`Completed`
            (`GameplayStatics.PlaySound2D` _sound_to_play 1.0 1.0 0.0 null null))))))
  (`|PlayMontage` (`self.Mesh`) "/Game/Characters/Enemies/EnemyAss/NormGhost/ghostnormal_Anim_Ghostarmature_Attac_Montage.ghostnormal_Anim_Ghostarmature_Attac_Montage"
    (:`then`
      (`CharacterMovementComponent.DisableMovement` (`self.CharacterMovement`))
      (`KismetSystemLibrary.Delay` 0.2)
      (`CharacterMovementComponent.SetMovementMode` (`self.CharacterMovement`) "MOVE_Walking" 0)
      (`GameplayStatics.SpawnEmitterAtLocation` "/Game/Characters/Devochka/FX/death.death" (`self.K2_GetActorLocation`))
      (`KismetSystemLibrary.Delay` 1.0)
      (set `/Game/Noises/VoicelinesController.Active Cue` null _returnvalue)
      (if (== (`self.Health`) 1)
        (`self.K2_DestroyActor`)))))

(fn `UserConstructionScript`
  (`parent.UserConstructionScript`))