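; BP_LittleGhost is an enemy character that reacts to slingshot, order and snow events, apparently overriding a shared parent.
; Slingshot and snow hits both play a one-shot squirrel throw animation as damage feedback, with a 2D sound call that shows no sound asset.
; The order event multiplies the ghost, repeatedly spawning AI copies of its own class at random reachable points nearby, raised above the ground.
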(event `/Game/Characters/Enemies/BP_EnemyBase.CustomReaction`
  ;[1 0.3247 0.3187] Рогатка
  (`SkeletalMeshComponent.PlayAnimation` (`self.Mesh`) "/Game/Characters/Enemies/EnemyAss/Squirrel/squirrel_Anim_metarig_Throw.squirrel_Anim_metarig_Throw" false) ; анимация получения урона
  (`GameplayStatics.PlaySound2D` null 1.0 1.0 0.0 null null) ; звук получения урона
)

(event `SpawnGhost`
  ;[1 1 1] Приказ
  (`AIBlueprintHelperLibrary.SpawnAIFromClass` "BP_LittleGhost_C" null (+ (`NavigationSystemV1.K2_GetRandomReachablePointInRadius` (`self.K2_GetActorLocation`) 300.0 null null) (* (`KismetMathLibrary.GetUpVector` (struct)) 100.0)) (struct) false null))

(event `/Game/Characters/Enemies/BP_EnemyBase.Prikazed Custom`
  ;[1 1 1] Приказ
  (for _ (range 3)
    (`self.SpawnGhost`)))

(event `/Game/Characters/Enemies/BP_EnemyBase.IsSnowed Custom`
  ;[0.3142 0.8536 1] Снег
  (`SkeletalMeshComponent.PlayAnimation` (`self.Mesh`) "/Game/Characters/Enemies/EnemyAss/Squirrel/squirrel_Anim_metarig_Throw.squirrel_Anim_metarig_Throw" false) ; анимация получения урона
  (`GameplayStatics.PlaySound2D` null 1.0 1.0 0.0 null null) ; звук получения урона
)

(fn `UserConstructionScript`
  (`parent.UserConstructionScript`))