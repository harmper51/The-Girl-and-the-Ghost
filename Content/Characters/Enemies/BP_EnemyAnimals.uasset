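; BP_EnemyAnimals is an animal enemy character that reacts to three effects: slingshot, order ("Prikaz") and snow.
; A slingshot reaction calls CustomReaction, then deals damage to the player rather than the animal.
; An order calls PrikazedCustom and destroys the animal after a short delay.
; Snow disables movement until a one-shot timer restores walking.
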(event `self.SlingshotReaction`
  ;[1 0.3156 0.3156] Рогатка
  (`self.CustomReaction`)
  (`GameplayStatics.ApplyDamage` (`GameplayStatics.GetPlayerCharacter` 0) 5.0))

(event `self.Prikazed`
  ;[1 1 1] Приказ
  (`self.Prikazed Custom`)
  (`KismetSystemLibrary.Delay` 0.5)
  (`self.K2_DestroyActor`))

(event `self.IsSnowed`
  ;[0.4767 0.9342 1] Снег
  (`CharacterMovementComponent.DisableMovement` (`self.CharacterMovement`))
  (`KismetSystemLibrary.K2_SetTimerDelegate` (delegate `NotSnowedAnymore`) 5.0))

(event `NotSnowedAnymore`
  ;[0.4767 0.9342 1] Снег
  (`CharacterMovementComponent.SetMovementMode` (`self.CharacterMovement`) "MOVE_Walking" 0))

(fn `UserConstructionScript`
  (`parent.UserConstructionScript`))