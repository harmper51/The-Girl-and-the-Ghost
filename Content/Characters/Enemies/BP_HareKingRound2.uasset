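; Hare King enemy actor for the second round, driven by the Prikazed event, which branches on whether it was hit.
; When hit, it scans the enemy collision's Enemies list and destroys itself and its WhoToDestroy target only if no Guardians remain.
; Otherwise it spawns a small particle burst, waits briefly, calls Round2 on the BP_hareCollisionPart1 actor, then destroys itself.
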(event `self.Prikazed`
  (if (`self.WasHit?`)
    (set `self.AreGuardiansAlive?` false)
    (for _array_element (`/Game/ThirdPerson/Blueprints/LevelPrototyping/BP_EnemyCollision.Enemies` (`self.As BP Enemy Collision`))
      (if (== (`GameplayStatics.GetObjectClass` _array_element) (`self.Guardians`))
        (set `self.AreGuardiansAlive?` true)
        (break)))
    (if (not (`self.AreGuardiansAlive?`))
      ;[1 1 1] Смерть
      (`self.K2_DestroyActor`)
      (`self.K2_DestroyActor` (`self.WhoToDestroy`)))
    (else
      (`GameplayStatics.SpawnEmitterAtLocation` "/Game/Characters/Devochka/FX/NewParticleSystem1.NewParticleSystem1" (`self.K2_GetActorLocation`) (struct) (0.1 0.1 0.1))
      (`KismetSystemLibrary.Delay` 1.0)
      (bind _returnvalue (`GameplayStatics.GetActorOfClass` "/Game/ThirdPerson/Blueprints/LevelPrototyping/BP_hareCollisionPart1.BP_hareCollisionPart1_C"))
      (`/Game/ThirdPerson/Blueprints/LevelPrototyping/BP_hareCollisionPart1.round 2` _returnvalue)
      (`self.K2_DestroyActor`))))

(fn `UserConstructionScript`
  (`parent.UserConstructionScript`))